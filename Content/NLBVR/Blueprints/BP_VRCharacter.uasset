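; VR character Blueprint that makes its left and right controller root components follow the tracked motion controllers.
; Each Tick queries both hands' Aim pose in Unreal world space through GetMotionControllerState and writes location and rotation straight to the matching root.
; An invalid state leaves that root unmoved and prints a per-hand error string.
; It has no other active logic.
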(event `self.ReceiveTick`
  (params (DeltaSeconds :type "Float (single-precision)"))
  (bind _motioncontrollerstate (`HeadMountedDisplayFunctionLibrary.GetMotionControllerState` self "UnrealWorldSpace" "Right" "Aim"))
  (bind (_bvalid _devicename _applicationinstanceid _xrspacetype _hand _trackingstatus _xrcontrollerposetype _controllerlocation _controllerrotation) (break `XRMotionControllerState` _motioncontrollerstate))
  (if _bvalid
    (`SceneComponent.K2_SetWorldLocationAndRotation` (`self.RightControllerRoot`) _controllerlocation (`KismetMathLibrary.Quat_Rotator` _controllerrotation) false false)
    (else
      (`KismetSystemLibrary.PrintString` "error right")))
  (bind _motioncontrollerstate_2 (`HeadMountedDisplayFunctionLibrary.GetMotionControllerState` self "UnrealWorldSpace" "Left" "Aim"))
  (bind (_bvalid_2 _devicename_2 _applicationinstanceid_2 _xrspacetype_2 _hand_2 _trackingstatus_2 _xrcontrollerposetype_2 _controllerlocation_2 _controllerrotation_2) (break `XRMotionControllerState` _motioncontrollerstate_2))
  (if _bvalid_2
    (`SceneComponent.K2_SetWorldLocationAndRotation` (`self.LeftControllerRoot`) _controllerlocation_2 (`KismetMathLibrary.Quat_Rotator` _controllerrotation_2) false false)
    (else
      (`KismetSystemLibrary.PrintString` "error left"))))

(fn `UserConstructionScript`)